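; BP_Background is a background actor for a side-scroller, apparently intended to follow the player, though that movement is currently disconnected.
; BeginPlay stores the player pawn's location as ReferencePoint, while Tick and the construction script are empty.
; Unconnected nodes hold experiments: following the character sprite, grid-snapping to the pawn at fixed depth, and a camera-relative parallax offset from ReferencePoint.
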(event `self.ReceiveBeginPlay`
  (set `self.ReferencePoint` (`self.K2_GetActorLocation` (`GameplayStatics.GetPlayerPawn` 0))))

(event `self.ReceiveTick`
  (params (DeltaSeconds :type "Float (single-precision)")))

(fn `UserConstructionScript`)